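; BP_HealthPickup is a health pickup that heals the player by a fixed amount and then destroys itself.
; When its Box component is overlapped, it takes the first BP_FirstPersonCharacter in the level without checking which actor overlapped.
; It calls HealPlayer only if that character is alive and not at full health, otherwise the pickup stays in place.
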(event OnComponentBeginOverlap(Box)
  (params (OverlappedComponent :type Primitive%20Component%20Object%20Reference) (OtherActor :type Actor%20Object%20Reference) (OtherComp :type Primitive%20Component%20Object%20Reference) (OtherBodyIndex :type Integer) (bFromSweep :type Boolean) (SweepResult :type Hit%20Result%20Structure%20%28by%20ref%29))
  ;[1 1 1] On player overlap add 10 HP
  (bind _outactors (Actor|GetAllActorsOfClass "/Game/FirstPerson/Blueprints/BP_FirstPersonCharacter.BP_FirstPersonCharacter_C"))
  (bind _output_get (Variables|Default|SetPlayer%20Character (Utilities|Array|Get(acopy) _outactors)))
  (if (and (not (Variables|/Game/FirstPerson/Blueprints/BP_FirstPersonCharacter.BP_FirstPersonCharacter_C|GetIsDead? (Variables|Default|GetPlayer%20Character))) (!= (Variables|/Game/FirstPerson/Blueprints/BP_FirstPersonCharacter.BP_FirstPersonCharacter_C|GetCurrentHealth (Variables|Default|GetPlayer%20Character)) (Variables|/Game/FirstPerson/Blueprints/BP_FirstPersonCharacter.BP_FirstPersonCharacter_C|GetMaxHealth (Variables|Default|GetPlayer%20Character))))
    (Default|HealPlayer _output_get 1e+01)
    (Actor|DestroyActor)))

(fn ConstructionScript)